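; BP_MeasuringTool is a spline-based measuring actor that displays the spline's length as text in a chosen metric or imperial unit.
; Tick and the construction script snap the last spline point to an optional AnchorActor, then update the label.
; The label converts and rounds the length, sitting just above the spline's midpoint.
; Helper functions zero or reset all tangents, refreshing the text manually because the construction script won't refire.
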(event `self.ReceiveTick`
  (params (DeltaSeconds :type "Float (single-precision)"))
  (`self.SnapToActor`)
  (`self.UpdateText`))

(fn `ResetTangents`
  (`self.SetTangents` (100.0 0.0 0.0)))

(fn `SetTangents`
  (params (Tangents :type "Vector Structure"))
  (bind _spline (`self.Spline`))
  (for _index (range (`SplineComponent.GetNumberOfSplinePoints` _spline))
    (`SplineComponent.SetTangentsAtSplinePoint` _spline _index Tangents Tangents "Local" true))
  (`self.UpdateText`) ; Update text when complete, since the\nconstruction script won't refire.
)

(fn `SnapToActor`
  (bind _anchoractor (`self.AnchorActor`))
  (bind _spline (`self.Spline`))
  (`/Engine/EditorBlueprintResources/StandardMacros.IsValid` _anchoractor
    (:`Is Valid`
      (`SplineComponent.SetLocationAtSplinePoint` _spline (- (`SplineComponent.GetNumberOfSplinePoints` _spline) 1) (`self.K2_GetActorLocation` _anchoractor) "World" true))))

(fn `UpdateText`
  (bind _value (`self.Value`))
  (bind _returnvalue (`SplineComponent.GetSplineLength` (`self.Spline`)))
  (`TextRenderComponent.K2_SetText` _value (`|FormatText` "{value}{unit}" (`KismetTextLibrary.Conv_DoubleToText` (* _returnvalue (select `/Game/MeasuringTool/EUnitTypes` (`self.UnitType`) :`NewEnumerator0` 1.0 :`NewEnumerator1` 0.01 :`NewEnumerator2` 1e-05 :`NewEnumerator3` 0.3937 :`NewEnumerator4` 0.010936 :`NewEnumerator5` 6e-06)) "HalfToEven" false true 1 324 2 2) (`KismetTextLibrary.Conv_StringToText` (`|GetEnumeratorNameAsString` (`self.UnitType`)))))
  (`SceneComponent.K2_SetWorldLocation` _value (+ (`SplineComponent.GetLocationAtDistanceAlongSpline` (`self.Spline`) (/ _returnvalue 2.0) "World") (0.0 0.0 16.0)) false false)
  (return))

(fn `UserConstructionScript`
  (`self.SnapToActor`)
  (`self.UpdateText`))

(fn `ZeroOutTangents`
  (`self.SetTangents` (0.0 0.0 0.0)))